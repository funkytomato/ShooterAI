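; Enemy shooter character that fights with a child-actor gun attached to its WeaponSocket and is driven by an AI controller.
; Shooting, reloading and aiming events drive the gun, anim instance, state flags and walk speed.
; Entering cover or being threatened runs the cover-shooting behavior tree; leaving cover restores the default tree.
; Damage plays a hit reaction, and death ragdolls the mesh, stops AI logic and ceases fire.
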(event Custom|StartShooting
  ;[1 1 1] Shooting
  (Default|StartShooting (Variables|Default|GetCurrentGun))
  (Variables|/Game/MyContent/Blueprints/EnemyShooter_AnimBP.EnemyShooter_AnimBP_C|SetIsShooting (Variables|Default|GetAnimInstance) true)
  (Variables|Default|SetIsShooting true))

(event Custom|StopShooting
  ;[1 1 1] Shooting
  (Default|StopShooting (Variables|Default|GetCurrentGun))
  (Variables|/Game/MyContent/Blueprints/EnemyShooter_AnimBP.EnemyShooter_AnimBP_C|SetIsShooting (Variables|Default|GetAnimInstance) false)
  (Variables|Default|SetIsShooting false))

(event Custom|Threatened
  (params (ThreatSource :type Vector))
  (bind _self self)
  (bind _returnvalue (AI|GetAIController _self))
  ;[1 1 1] Threatened
  (Variables|Default|SetIsUnderFire true)
  (Development|PrintString "Enemy is Threatened")
  (AI|RunBehaviorTree _returnvalue "/Game/MyContent/AI/EnemyShootFromCover_BT.EnemyShootFromCover_BT")
  (AI|SetFocalPoint _returnvalue ThreatSource))

(event Custom|StartAiming
  ;[1 1 1] Aiming (Ironsights)
  (Variables|Default|SetIsADS true)
  (Variables|/Script/Engine.CharacterMovementComponent|SetMaxWalkSpeed (Variables|Character|GetCharacterMovement) 2.7e+02))

(event Custom|StopAiming
  ;[1 1 1] Aiming (Ironsights)
  (Variables|Default|SetIsADS false)
  (Variables|/Script/Engine.CharacterMovementComponent|SetMaxWalkSpeed (Variables|Character|GetCharacterMovement) 6e+02))

(event Custom|EnterCover
  ;[1 1 1] Cover - Enter and Leave
  (Variables|Default|SetIsADS true)
  (Variables|Default|SetIsInCover true)
  (Character|Crouch)
  (AI|RunBehaviorTree (AI|GetAIController self) "/Game/MyContent/AI/EnemyShootFromCover_BT.EnemyShootFromCover_BT"))

(event Custom|LeaveCover
  ;[1 1 1] Cover - Enter and Leave
  (Variables|Default|SetIsInCover false)
  (Character|UnCrouch)
  (AI|RunBehaviorTree (AI|GetAIController self) "/Game/MyContent/AI/Shooter_BT.Shooter_BT")
  (Development|PrintString "Leave cover"))

(event Custom|Reload
  ;[1 1 1] Reload
  (if (Variables|Default|GetIsADS)
    (Animation|Montage|MontagePlay (Variables|Default|GetAnimInstance) "/Game/AnimStarterPack/Reload_Rifle_Ironsights_Montage.Reload_Rifle_Ironsights_Montage" 1.0 "MontageLength" 0.0 true)
    (Default|Reload (Variables|Default|GetCurrentGun))
    (else
      (Animation|Montage|MontagePlay (Variables|Default|GetAnimInstance) "/Game/AnimStarterPack/Reload_Rifle_Hip_Montage.Reload_Rifle_Hip_Montage" 1.0 "MontageLength" 0.0 true)
      (Default|Reload (Variables|Default|GetCurrentGun)))))

(event EventBeginPlay
  ;[1 1 1] BeginPlay - Animinstance Ref, GunMaster Ref and ShooterAIController Ref
  (Utilities|FlowControl|Sequence
    (:then_0
      (bind _asenemy_shooter_anim_bp (Utilities|Casting|CastToEnemyShooter_AnimBP (Components|SkeletalMesh|GetAnimInstance (Variables|Character|GetMesh))))
      (Variables|Default|SetAnimInstance _asenemy_shooter_anim_bp))
    (:then_1
      (bind _asgun_master_bp (Utilities|Casting|CastToGunMaster_BP (Variables|/Script/Engine.ChildActorComponent|GetChildActor (Variables|Default|GetGun))))
      (Variables|Default|SetCurrentGun _asgun_master_bp))
    (:then_2
      (bind _asshooter_aicontroller (Utilities|Casting|CastToShooterAIController (AI|GetAIController self)))
      (bind _output_get (Variables|Default|SetPawnAIController _asshooter_aicontroller))
      (Development|PrintString (Utilities|GetDisplayName _output_get)))))

(event Game|Damage|EventAnyDamage
  (params (Damage :type Float%20%28single-precision%29) (DamageType :type Damage%20Type%20Object%20Reference) (InstigatedBy :type Controller%20Object%20Reference) (DamageCauser :type Actor%20Object%20Reference))
  ;[1 1 1] AnyDamage
  (bind _output_get (Variables|Default|SetHealth (- (Variables|Default|GetHealth) Damage)))
  (if (<= _output_get 0.0)
    (Physics|SetSimulatePhysics (Variables|Character|GetMesh) true)
    (AI|Logic|StopLogic (Variables|/Script/AIModule.AIController|GetBrainComponent (AI|GetAIController self)) "")
    (Collision|SetCollisionEnabled (Variables|Default|GetCapsuleComponent) "NoCollision")
    (CallFunction|StopShooting)
    (else
      (Animation|Montage|MontagePlay (Variables|Default|GetAnimInstance) "/Game/AnimStarterPack/Hit_React_1_Montage.Hit_React_1_Montage" 1.0 "MontageLength" 0.0 true))))

(fn ConstructionScript
  (Transformation|AttachComponentToComponent (Variables|Default|GetGun) (Variables|Character|GetMesh) "WeaponSocket" "SnapToTarget" "SnapToTarget" "SnapToTarget" true))