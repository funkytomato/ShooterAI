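; Fully automatic gun Blueprint that keeps firing projectiles while shooting is active.
; StartShooting calls the parent, fires one projectile immediately, then starts a looping timer that repeats FireProjectile every FireRate seconds.
; StopShooting calls the parent and clears that timer by its stored handle.
; A debug string prints when firing starts.
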(event EventBeginPlay
  (|CallParentFunction) ; This node is disabled and will not be called.\nDrag off pins to build functionality.
)

(event EventStartShooting
  (|CallParentFunction)
  (CallFunction|FireProjectile)
  (bind _returnvalue (Utilities|Time|SetTimerbyFunctionName 0 "FireProjectile" (Variables|Default|GetFireRate) true))
  (Variables|Default|SetGunTimer _returnvalue)
  (Development|PrintString "FullyAutomatic firing"))

(event EventStopShooting
  (|CallParentFunction)
  (Utilities|Time|ClearandInvalidateTimerbyHandle (Variables|Default|GetGunTimer)))

(fn ConstructionScript
  (|CallParentFunction))