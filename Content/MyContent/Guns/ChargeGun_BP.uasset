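; ChargeGun_BP is a chargeable gun, extending a parent weapon, whose projectile speed scales with how long the shot charges.
; StartShooting plays the ChargeWeapon timeline at a rate set by ChargeTime to drive CurrentCharge, automatically calling StopShooting at full charge.
; StopShooting fires if charge passes a minimum, then reverses the timeline; recharging waits until charge drains low.
; FireProjectile scales BulletSpeed by charge around the parent call, then resets it to a hardcoded default.
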(event EventBeginPlay
  (|CallParentFunction) ; This node is disabled and will not be called.\nDrag off pins to build functionality.
)

(event Collision|EventActorBeginOverlap
  (params (OtherActor :type Actor%20Object%20Reference)))

(event EventTick
  (params (DeltaSeconds :type Float%20%28single-precision%29)))

(event EventStartShooting
  (|CallParentFunction)
  (if (and (not (Variables|Default|GetIsCharging?)) (<= (Variables|Default|GetCurrentCharge) 0.2))
    (Variables|Default|SetIsCharging? true)
    (Components|Timeline|SetPlayRate (Variables|Default|GetChargeWeapon) (/ 1.0 (Variables|Default|GetChargeTime)))
    (bind _weaponcharge (Timeline|ChargeWeapon Play)
      (:Update
        (bind _output_get (Variables|Default|SetCurrentCharge (Math|Float|Clamp(Float) _weaponcharge)))
        (if (>= _output_get 1.0)
          (CallFunction|StopShooting))))))

(event EventStopShooting
  (|CallParentFunction)
  (if (and (Variables|Default|GetIsCharging?) (>= (Variables|Default|GetCurrentCharge) 0.2))
    (CallFunction|FireProjectile))
  (Variables|Default|SetIsCharging? false)
  (Components|Timeline|SetPlayRate (Variables|Default|GetChargeWeapon) 1.0)
  (bind _weaponcharge (Timeline|ChargeWeapon Reverse)
    (:Update
      (bind _output_get (Variables|Default|SetCurrentCharge (Math|Float|Clamp(Float) _weaponcharge)))
      (if (>= _output_get 1.0)
        (CallFunction|StopShooting)))))

(fn ConstructionScript
  (|CallParentFunction))

(fn FireProjectile
  (Variables|Default|SetBulletSpeed (* (Variables|Default|GetBulletSpeed) (Variables|Default|GetCurrentCharge)))
  (|CallParentFunction)
  (Variables|Default|SetBulletSpeed 3e+03))