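; Base gun Blueprint, used as a child actor of a ThirdPersonCharacter, that handles firing, reloading from reserve ammo and threatening nearby targets.
; StartShooting fires once; hitscan mode line-traces from the follow camera and pushes physics objects, without consuming ammo.
; Each shot also sphere-traces from the muzzle, with threat level as radius, calling Threatened on a ShooterCharacter or EnemyShooter hit.
; Non-hitscan mode only threat-traces and decrements ammo, as projectile spawning is disconnected.
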(event Custom|StartShooting
  (Development|PrintString "Start shooting")
  (Variables|Default|SetIsFiring true)
  (CallFunction|FireProjectile))

(event Custom|StopShooting
  (Development|PrintString "Stop shooting")
  (Variables|Default|SetIsFiring false))

(event EventBeginPlay
  (bind _asthird_person_character (Utilities|Casting|CastToThirdPersonCharacter (Actor|GetParentActor)))
  (Variables|Default|SetGunOwner _asthird_person_character))

(fn ConstructionScript)

(fn FireProjectile
  (bind _gunowner (Variables|Default|GetGunOwner))
  (bind _followcamera (Variables|/Game/ThirdPersonBP/Blueprints/ThirdPersonCharacter.ThirdPersonCharacter_C|GetFollowCamera _gunowner))
  (bind _returnvalue (Transformation|GetWorldRotation _followcamera))
  (bind _returnvalue_2 (Math|Vector|GetForwardVector _returnvalue))
  (if (Variables|Default|GetIsHitScan)
    (if (> (Variables|Default|GetAmmoCount) 0)
      (if true
        (CallFunction|ThreatTrace (Variables|Default|GetThreatLevel))
        (Variables|Default|SetGunDirection _returnvalue_2)
        (bind _outhit (Collision|LineTraceByChannel (Transformation|GetWorldLocation _followcamera) (+ (Transformation|GetWorldLocation _followcamera) (* _returnvalue_2 2e+03)) "TraceTypeQuery1" false 0 "ForDuration"))
        (if (.bBlockingHit (Collision|BreakHitResult _outhit))
          (if (Physics|IsSimulatingPhysics (.HitComponent (Collision|BreakHitResult _outhit)) "None")
            (Physics|AddImpulseatLocation (.HitComponent (Collision|BreakHitResult _outhit)) (* (Variables|Default|GetGunDirection) 2e+05) (.ImpactPoint (Collision|BreakHitResult _outhit)) "None")))))
    (elif (> (Variables|Default|GetAmmoCount) 0)
      (CallFunction|ThreatTrace (Variables|Default|GetThreatLevel))
      (Math|Integer|DecrementInt (Variables|Default|GetAmmoCount)))))

(fn ThreatTrace
  (params (ThreatValue :type Float%20%28single-precision%29))
  (bind _muzzleref (Variables|Default|GetMuzzleRef))
  (bind _returnvalue (Transformation|GetWorldLocation _muzzleref))
  (bind _outhit (Collision|SphereTraceByChannel _returnvalue (+ _returnvalue (* (Math|Vector|GetForwardVector (Transformation|GetWorldRotation (Variables|/Game/ThirdPersonBP/Blueprints/ThirdPersonCharacter.ThirdPersonCharacter_C|GetFollowCamera (Variables|Default|GetGunOwner)))) (Variables|Default|GetRange))) ThreatValue "TraceTypeQuery2" false (Utilities|Array|MakeArray (Variables|Default|GetGunOwner)) "ForDuration" true "(R=0.009268,G=0.021773,B=1.000000,A=1.000000)" "(R=0.000000,G=0.795357,B=1.000000,A=1.000000)"))
  (if (.bblockinghit _outhit)
    (bind _asshooter_character (Utilities|Casting|CastToShooterCharacter (.hitactor _outhit))
      (:then
        (Default|Threatened _asshooter_character))
      (:CastFailed
        (bind _asenemy_shooter (Utilities|Casting|CastToEnemyShooter (.hitactor _outhit)))
        (Default|Threatened _asenemy_shooter)))))

(fn Reload
  (Variables|Default|SetBulletDifference (- (Variables|Default|GetClipSize) (Variables|Default|GetAmmoCount)))
  (if (>= (Variables|Default|GetAmmoMax) (Variables|Default|GetBulletDifference))
    (Variables|Default|SetAmmoCount (Variables|Default|GetClipSize))
    (Variables|Default|SetAmmoMax (- (Variables|Default|GetAmmoMax) (Variables|Default|GetBulletDifference)))
    (else
      (Variables|Default|SetAmmoCount (+ (Variables|Default|GetAmmoCount) (Variables|Default|GetAmmoMax)))
      (Variables|Default|SetAmmoMax 0))))